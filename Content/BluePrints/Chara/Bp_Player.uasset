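; Player character Blueprint that handles camera look, camera-relative movement, sprinting and a saber attack.
; Movement follows control yaw and respects CanInputMove; sideways input also stops during slot animations, forward input while falling.
; Attack plays the saber montage only when ComboCount is zero, and EndCombo resets it.
; SetComboInputFlg stores a combo-input flag unused here, and jump logic is disconnected.
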(event EventBeginPlay
  (bind _returnvalue (Game|GetPlayerCameraManager 0))
  (Variables|/Script/Engine.PlayerCameraManager|SetViewPitchMax _returnvalue 3e+01)
  (Variables|/Script/Engine.PlayerCameraManager|SetViewPitchMin _returnvalue -2e+01))

(event Input|ActionEvents|InputActionJump
  (params (Key :type Key%20Structure :default "None")))

(event Input|ActionEvents|InputActionAttack
  (params (Key :type Key%20Structure :default "None"))
  (:Pressed
    (CallFunction|ExecAttack)))

(event Input|ActionEvents|InputActionaccel
  (params (Key :type Key%20Structure :default "None"))
  (bind _charactermovement (Variables|Character|GetCharacterMovement))
  (:Pressed
    (Variables|/Script/Engine.CharacterMovementComponent|SetMaxWalkSpeed _charactermovement 1e+03))
  (:Released
    (Variables|/Script/Engine.CharacterMovementComponent|SetMaxWalkSpeed _charactermovement 6e+02)))

(event Input|AxisEvents|InputAxisLookUp/DownGamepad
  (params (AxisValue :type Float%20%28single-precision%29))
  (Pawn|Input|AddControllerPitchInput (* AxisValue 5e+01 (Utilities|Time|GetWorldDeltaSeconds))))

(event Input|AxisEvents|InputAxisLookUp/DownMouse
  (params (AxisValue :type Float%20%28single-precision%29))
  (Pawn|Input|AddControllerPitchInput AxisValue))

(event Input|AxisEvents|InputAxisTurnRight/LeftMouse
  (params (AxisValue :type Float%20%28single-precision%29))
  (Pawn|Input|AddControllerYawInput AxisValue))

(event Input|AxisEvents|InputAxisMoveForward/Backward
  (params (AxisValue :type Float%20%28single-precision%29))
  (if (not (or (not (Variables|Default|GetCanInputMove)) (AI|Components|NavMovement|IsFalling (Variables|Character|GetCharacterMovement))))
    (Pawn|Input|AddMovementInput (Math|Vector|GetForwardVector (Math|Rotator|MakeRotator 0.0 0.0 (.yaw (Pawn|GetControlRotation :!class /Script/Engine.Pawn)))) AxisValue false)))

(event Input|AxisEvents|InputAxisMoveRight/Left
  (params (AxisValue :type Float%20%28single-precision%29))
  (if (not (or (Class|AnimInstance|IsPlayingSlotAnimation (Components|SkeletalMesh|GetAnimInstance (Variables|Character|GetMesh)) 0 "DefalutGroup.DefalutSlot") (not (Variables|Default|GetCanInputMove))))
    (Pawn|Input|AddMovementInput (Math|Vector|GetRightVector (Math|Rotator|MakeRotator 0.0 0.0 (.yaw (Pawn|GetControlRotation :!class /Script/Engine.Pawn)))) AxisValue false)))

(event Input|AxisEvents|InputAxisTurnRight/LeftGamepad
  (params (AxisValue :type Float%20%28single-precision%29))
  (Pawn|Input|AddControllerYawInput (* AxisValue 5e+01 (Utilities|Time|GetWorldDeltaSeconds))))

(fn ConstructionScript)

(fn SetComboInputFlg
  (params (Flg :type Boolean))
  (Variables|Default|SetComboInputEnableFlg Flg))

(fn ExecAttack
  (if (<= (Variables|Default|GetComboCount) 0)
    (Animation|Montage|MontagePlay (Components|SkeletalMesh|GetAnimInstance (Variables|Character|GetMesh)) "/Game/BluePrints/Chara/AnimAssets/AM_Player_Saber.AM_Player_Saber" 1.0 "MontageLength" 0.0 true)
    (Variables|Default|SetComboCount 1)))

(fn EndCombo
  (Variables|Default|SetComboCount 0))